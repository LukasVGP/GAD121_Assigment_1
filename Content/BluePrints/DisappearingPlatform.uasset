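; DisappearingPlatform is a platform that vanishes shortly after the player touches it and later returns.
; An overlap on PlayerTrigger by the third-person character starts a timed sequence that hides PlatformMesh and disables its collision, then restores both after a longer delay.
; A DoOnce gate blocks retriggering until the platform has reappeared.
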(event OnComponentBeginOverlap(PlayerTrigger)
  (params (OverlappedComponent :type Primitive%20Component%20Object%20Reference) (OtherActor :type Actor%20Object%20Reference) (OtherComp :type Primitive%20Component%20Object%20Reference) (OtherBodyIndex :type Integer) (bFromSweep :type Boolean) (SweepResult :type Hit%20Result%20Structure%20%28by%20ref%29))
  (Utilities|Casting|CastToBP_ThirdPersonCharacter OtherActor)
  (Utilities|FlowControl|DoOnce false :!label _label
    (:Completed
      (Utilities|FlowControl|Delay 1.0)
      (Rendering|SetVisibility (Variables|Default|GetPlatformMesh) false false)
      (Collision|SetCollisionEnabled (Variables|Default|GetPlatformMesh) "NoCollision")
      (Utilities|FlowControl|Delay 5.0)
      (Rendering|SetVisibility (Variables|Default|GetPlatformMesh) true false)
      (Collision|SetCollisionEnabled (Variables|Default|GetPlatformMesh) "QueryAndPhysics")
      (goto _label Reset))))

(fn ConstructionScript)